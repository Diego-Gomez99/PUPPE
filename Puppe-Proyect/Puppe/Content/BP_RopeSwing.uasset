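; BP_RopeSwing is a rope the player character can grab and swing on.
; It caches the third-person character at start, and when its box trigger is overlapped while the jump key or gamepad face button is held, it flags the player as on-rope, passes itself as the rope and attaches them.
; Releasing the jump action detaches the player and clears the on-rope state and rope reference.
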(event `self.ReceiveBeginPlay`
  (bind _asbp_third_person_character (cast `/Game/ThirdPerson/Blueprints/BP_ThirdPersonCharacter` (`GameplayStatics.GetPlayerCharacter` 0)))
  (set `self.Player` _asbp_third_person_character))

(event `InputAction|JumpAction`
  (params (Key :type "Key Structure"))
  (bind _player (`self.Player`))
  (:`Released`
    (`self.DettachPlayer`)
    (`PuppeCharacter.SetIsOnRope` _player false)
    (`/Game/ThirdPerson/Blueprints/BP_ThirdPersonCharacter.SetRope` _player null)))

(event `self.BoxComp.OnComponentBeginOverlap`
  (params (OverlappedComponent :type "PrimitiveComponent Object Reference") (OtherActor :type "Actor Object Reference") (OtherComp :type "PrimitiveComponent Object Reference") (OtherBodyIndex :type Integer) (bFromSweep :type Boolean) (SweepResult :type "HitResult Structure (by ref)"))
  (bind _returnvalue (`GameplayStatics.GetPlayerController` 0))
  (bind _player (`self.Player`))
  (if (or (`PlayerController.IsInputKeyDown` _returnvalue "SpaceBar") (`PlayerController.IsInputKeyDown` _returnvalue "Gamepad_FaceButton_Bottom"))
    (`PuppeCharacter.SetIsOnRope` _player true)
    (`/Game/ThirdPerson/Blueprints/BP_ThirdPersonCharacter.SetRope` _player self)
    (`self.AttachActor`)))

(fn `UserConstructionScript`)