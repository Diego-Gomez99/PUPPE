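; Pushable world object that, when interacted with, snaps the player to a push spot and starts pushing through the player's PushComponent.
; Push spots come from the PushTransform array, shown as arrows by the construction script, and the nearest within the component's PushRange is chosen.
; Capsule and line traces check standing room, walkable floor and obstructions before the teleport, with debug drawing and printed failure reasons.
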(event `/Game/Interactive_Interface/BP_InteractInterface.OnInteracted`
  (params (Player :type "/Game/ThirdPerson/Blueprints/BP_ThirdPersonCharacter Object Reference"))
  (`self.HandleInteraction` Player))

(fn `FindClosestPushTransformIndex`
  (params (CharacterLocation :type "Vector2D Structure") (PushRange :type "Float (double-precision)"))
  (returns (BestIndex :type Integer))
  (locals (CurrentTransformIndex :type Integer) (CurrentDistanceSq :type "Float (double-precision)" :default 0.0) (ClosestDistanceSq :type "Float (double-precision)") (ClosestTransformIndex :type Integer :default -1))
  (for (_array_element _array_index) (`self.PushTransform`)
    (set `local.CurrentTransformIndex` _array_index)
    (set `local.CurrentDistanceSq` (`KismetMathLibrary.DistanceSquared2D` (`KismetMathLibrary.Conv_VectorToVector2D` (`KismetMathLibrary.TransformLocation` (`self.GetTransform`) (.location _array_element))) (`local.CharacterLocation`)))
    (if (< (`local.CurrentDistanceSq`) (`KismetMathLibrary.Square` (`local.PushRange`)))
      (if (or (< (`local.CurrentDistanceSq`) (`local.ClosestDistanceSq`)) (< (`local.ClosestTransformIndex`) 0))
        (set `local.ClosestTransformIndex` (`local.CurrentTransformIndex`))
        (set `local.ClosestDistanceSq` (`local.CurrentDistanceSq`)))))
  (return (`local.ClosestTransformIndex`)))

(fn `HandleInteraction`
  (params (Player :type "/Game/ThirdPerson/Blueprints/BP_ThirdPersonCharacter Object Reference"))
  (locals (PushComponent :type "/Game/Interact_Objs/Pushable/PushComponent Object Reference") (NewCharaterLocation :type "Transform Structure"))
  (bind _returnvalue (`self.GetComponentByClass` Player "/Game/Interact_Objs/Pushable/PushComponent.PushComponent_C"))
  (bind _newcharaterlocation_location (`KismetMathLibrary.BreakTransform` (`local.NewCharaterLocation`)))
  (bind _newcharaterlocation_location_2 (`KismetMathLibrary.BreakTransform` (`local.NewCharaterLocation`)))
  (bind (_returnvalue_location _returnvalue_rotation _returnvalue_scale) (`KismetMathLibrary.BreakTransform` (`self.GetTransform` (`local.Player`))))
  (bind _capsulecomponent (`Character.CapsuleComponent` (`local.Player`)))
  (`/Engine/EditorBlueprintResources/StandardMacros.IsValid` Player
    (:`Is Valid`
      (`/Engine/EditorBlueprintResources/StandardMacros.IsValid` _returnvalue
        (:`Is Valid`
          (set `local.PushComponent` _returnvalue)
          (bind _bestindex (`self.FindClosestPushTransformIndex` (`KismetMathLibrary.Conv_VectorToVector2D` (`self.K2_GetActorLocation` (`local.Player`))) (`/Game/Interact_Objs/Pushable/PushComponent.PushRange` (`local.PushComponent`))))
          (if (>= _bestindex 0)
            (bind (_returnvalue_location_2 _returnvalue_rotation_2) (`KismetMathLibrary.BreakTransform` (`KismetMathLibrary.ComposeTransforms` (`|GetArrayItem` (`self.PushTransform`) _bestindex) (`self.GetTransform`))))
            (set `local.NewCharaterLocation` (`KismetMathLibrary.MakeTransform` (+ _returnvalue_location_2 (`KismetMathLibrary.MakeVector` 0.0 0.0 (`CapsuleComponent.GetScaledCapsuleHalfHeight` (`Character.CapsuleComponent` (`local.Player`))))) _returnvalue_rotation_2 _returnvalue_scale))
            ;[1 1 1] Verify if the player can stand in the room to push
            (bind _outhit (`KismetSystemLibrary.CapsuleTraceSingle` :`Start` (+ _newcharaterlocation_location_2 (0.0 0.0 70.0)) :`End` (- _newcharaterlocation_location_2 (0.0 0.0 100.0)) :`Radius` (`CapsuleComponent.GetScaledCapsuleRadius` _capsulecomponent) :`HalfHeight` (`CapsuleComponent.GetScaledCapsuleHalfHeight` _capsulecomponent) :`TraceChannel` "TraceTypeQuery1" :`DrawDebugType` "ForDuration"))
            (if (not (`.bInitialOverlap` (`GameplayStatics.BreakHitResult` _outhit)))
              (if (< (`CharacterMovementComponent.K2_GetWalkableFloorZ` (`Character.CharacterMovement` (`local.Player`))) (.z (`.ImpactNormal` (`GameplayStatics.BreakHitResult` _outhit))))
                (bind (_outhit_2 _returnvalue_2) (`KismetSystemLibrary.LineTraceSingle` (`self.K2_GetActorLocation`) _newcharaterlocation_location "TraceTypeQuery1" false (`|MakeArray` (`local.Player`) :!type "Actor Object Reference") "ForDuration" true (struct :`R` 1.0 :`G` 0.857417 :`B` 0.119745 :`A` 1.0) (struct :`R` 0.017018 :`G` 0.555887 :`B` 1.0 :`A` 1.0)))
                (if (not _returnvalue_2)
                  (`self.K2_SetActorTransform` (`local.Player`) (`local.NewCharaterLocation`) false false)
                  (`/Game/Interact_Objs/Pushable/PushComponent.BeginPush` (`local.PushComponent`) self)
                  (else
                    (`KismetSystemLibrary.PrintString` "Object between player and pushable Obj" true true (struct :`R` 1.0 :`B` 0.079394 :`A` 1.0))))
                (else
                  (`KismetSystemLibrary.PrintString` "Floor is not Walkable" true true (struct :`R` 1.0 :`B` 0.064177 :`A` 1.0) 3.0)))
              (else
                (`KismetSystemLibrary.PrintString` "No room to Stand" true true (struct :`R` 1.0 :`B` 0.064177 :`A` 1.0) 3.0)))
            (else
              (`KismetSystemLibrary.PrintString` "Push Transform not found"))))
        (:`Is Not Valid`
          (`KismetSystemLibrary.PrintString` "Component Not Valid" true true (struct :`R` 1.0 :`B` 0.092125 :`A` 1.0) 3.0))))
    (:`Is Not Valid`
      (`KismetSystemLibrary.PrintString` "Character Not Valid" true true (struct :`R` 1.0 :`B` 0.074582 :`A` 1.0) 3.0))))

(fn `UserConstructionScript`
  ;[0 0 0] Add Arrow as Widget to locate the character and start pushing
  (for _array_element (`self.PushTransform`)
    (`AddComponent|NODE_AddArrowComponent-0` :`RelativeTransform` _array_element)))