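; Ladder actor that the third-person character can get on and off through interaction.
; OnInteracted stores the player, calls SetOnLadder and registers the ladder with the character.
; Releasing Interact calls SetOffLadder unless a montage check blocks it, as does leaving the box, unconditionally.
; Box and sphere overlaps flag proximity, and the construction script adds an arrow component per LadderTransform entry.
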(event `InputAction|Interact`
  (params (Key :type "Key Structure"))
  (:`Released`
    (bind _returnvalue (`self.CheckIfAMontageIsPlaying`))
    (if (not _returnvalue)
      (`self.SetOffLadder`))))

(event `self.ReceiveBeginPlay`
  (bind _asbp_third_person_character (cast `/Game/ThirdPerson/Blueprints/BP_ThirdPersonCharacter` (`GameplayStatics.GetPlayerCharacter` 0)))
  (bind _output_get (set `self.As BP Third Person Character` _asbp_third_person_character))
  (`self.SetPlayerCharacter` _output_get))

(event `/Game/Interactive_Interface/BP_InteractInterface.OnInteracted`
  (params (Player :type "/Game/ThirdPerson/Blueprints/BP_ThirdPersonCharacter Object Reference"))
  (`self.SetPlayerCharacter` Player)
  (`self.SetOnLadder`)
  (`/Game/ThirdPerson/Blueprints/BP_ThirdPersonCharacter.SetLadderBP` (`self.As BP Third Person Character`) self))

(event `self.Box.OnComponentBeginOverlap`
  (params (OverlappedComponent :type "PrimitiveComponent Object Reference") (OtherActor :type "Actor Object Reference") (OtherComp :type "PrimitiveComponent Object Reference") (OtherBodyIndex :type Integer) (bFromSweep :type Boolean) (SweepResult :type "HitResult Structure (by ref)"))
  (cast `/Game/ThirdPerson/Blueprints/BP_ThirdPersonCharacter` OtherActor)
  (set `self.bIsNearLadder` true))

(event `self.Box.OnComponentEndOverlap`
  (params (OverlappedComponent :type "PrimitiveComponent Object Reference") (OtherActor :type "Actor Object Reference") (OtherComp :type "PrimitiveComponent Object Reference") (OtherBodyIndex :type Integer))
  (cast `/Game/ThirdPerson/Blueprints/BP_ThirdPersonCharacter` OtherActor)
  (set `self.bIsNearLadder` false)
  (`self.SetOffLadder`))

(event `self.Sphere.OnComponentBeginOverlap`
  (params (OverlappedComponent :type "PrimitiveComponent Object Reference") (OtherActor :type "Actor Object Reference") (OtherComp :type "PrimitiveComponent Object Reference") (OtherBodyIndex :type Integer) (bFromSweep :type Boolean) (SweepResult :type "HitResult Structure (by ref)"))
  (cast `/Game/ThirdPerson/Blueprints/BP_ThirdPersonCharacter` OtherActor)
  (set `self.bIsNearLadder` true))

(fn `UserConstructionScript`
  (for _array_element (`self.LadderTransform`)
    (`AddComponent|NODE_AddArrowComponent-0` :`RelativeTransform` _array_element)))